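; Racing game mode that runs a timed race, deciding win or loss by the finish line and a time limit.
; BeginPlay binds to the crossed event of finish-line BP_Checkpoint actors, then runs a delayed countdown before starting the race timer.
; Timer expiry loses, while the win event clears the timer; both call GameFinish.
; Countdown, start and result feedback are only printed strings.
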(event `self.ReceiveBeginPlay`
  (`|ExecutionSequence`
    (:`then_0`
      (bind _outactors (`GameplayStatics.GetAllActorsOfClass` "/Game/RacingGame/Checkpoints/BP_Checkpoint.BP_Checkpoint_C"))
      (for _array_element _outactors
        (if (`/Game/RacingGame/Checkpoints/BP_Checkpoint.isFinishLine` _array_element)
          (add `/Game/RacingGame/Checkpoints/BP_Checkpoint.OnCheckpointCrossed` _array_element (`|CreateDelegate` :!event `Win_CrossTheFinishLine`)))))
    (:`then_1`
      (`self.Start Countdown`))))

(event `Start Countdown`
  (`KismetSystemLibrary.PrintString` "Start Countdown")
  (`KismetSystemLibrary.Delay` (`self.StartCountdownDuration`))
  (`self.Game Start`))

(event `Game Start`
  (`KismetSystemLibrary.PrintString` "Game Start")
  (bind _returnvalue (`KismetSystemLibrary.K2_SetTimerDelegate` (delegate `Lose_OutOfTime`) (`self.StartTimerDuration`)))
  (set `self.Time Remainig TImer` _returnvalue))

(event `Lose_OutOfTime`
  (`self.Game Finish` false))

(event `Win_CrossTheFinishLine`
  (`KismetSystemLibrary.K2_ClearAndInvalidateTimerHandle` (`self.Time Remainig TImer`))
  (`self.Game Finish` true))

(event `Game Finish`
  (params (Win :type Boolean))
  (`KismetSystemLibrary.PrintString` (`KismetMathLibrary.SelectString` "You win" "You lose" Win)))

(fn `UserConstructionScript`)